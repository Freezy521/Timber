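; Crumbling 2D platform that cracks and disappears shortly after a character steps on it, then respawns.
; A box trigger overlap swaps the Paper2D sprite to a cracked version, waits briefly, then hides it and disables its collision.
; When any overlap with the box ends, a longer delay restores the original sprite, visibility and collision, with no check on which actor left.
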(event `self.Box.OnComponentBeginOverlap`
  (params (OverlappedComponent :type "PrimitiveComponent Object Reference") (OtherActor :type "Actor Object Reference") (OtherComp :type "PrimitiveComponent Object Reference") (OtherBodyIndex :type Integer) (bFromSweep :type Boolean) (SweepResult :type "HitResult Structure (by ref)"))
  (cast `Character` OtherActor)
  (`PaperSpriteComponent.SetSprite` (`self.PaperSprite`) "/Game/2DSideScrollerBP/Test/cracked_platform_Sprite_0.cracked_platform_Sprite_0")
  (`KismetSystemLibrary.Delay` 0.3)
  (`SceneComponent.SetVisibility` (`self.PaperSprite`) false false)
  (`PrimitiveComponent.SetCollisionEnabled` (`self.PaperSprite`) "NoCollision"))

(event `self.Box.OnComponentEndOverlap`
  (params (OverlappedComponent :type "PrimitiveComponent Object Reference") (OtherActor :type "Actor Object Reference") (OtherComp :type "PrimitiveComponent Object Reference") (OtherBodyIndex :type Integer))
  (`KismetSystemLibrary.Delay` 1.0)
  (`PaperSpriteComponent.SetSprite` (`self.PaperSprite`) "/Game/2DSideScrollerBP/Test/platform_Sprite_0.platform_Sprite_0")
  (`SceneComponent.SetVisibility` (`self.PaperSprite`) true false)
  (`PrimitiveComponent.SetCollisionEnabled` (`self.PaperSprite`) "QueryAndPhysics"))

(fn `UserConstructionScript`)