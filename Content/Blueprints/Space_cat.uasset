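; Space cat enemy for a 2D side-scroller that knocks back and briefly stuns the player on contact.
; An InterpToMovement component moves it between relative points PointA and PointB, set in the Construction Script.
; A box hit by the side-scroller character switches to the attack flipbook, plays a screech and launches the character up and away.
; It shows a stun message and disables player input, restoring input and the default flipbook after a short delay.
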(event `self.ReceiveBeginPlay`)

(event `self.Box.OnComponentHit`
  (params (HitComponent :type "PrimitiveComponent Object Reference") (OtherActor :type "Actor Object Reference") (OtherComp :type "PrimitiveComponent Object Reference") (NormalImpulse :type "Vector Structure") (Hit :type "HitResult Structure (by ref)"))
  (bind _returnvalue (`GameplayStatics.GetPlayerController` 0))
  (bind _returnvalue_2 (`GameplayStatics.GetPlayerCharacter` 0))
  (bind _as2dside_scroller_character (cast `/Game/2DSideScrollerBP/Blueprints/2DSideScrollerCharacter` OtherActor))
  (`PaperFlipbookComponent.SetFlipbook` (`self.PaperFlipbook`) "/Game/Assets/Space_Cyat/Attack/Space_Cat_Attack.Space_Cat_Attack")
  (`Character.LaunchCharacter` _as2dside_scroller_character (`KismetMathLibrary.MakeVector` (.x (* (`KismetMathLibrary.GetDirectionUnitVector` (`self.K2_GetActorLocation` (`GameplayStatics.GetPlayerCharacter` 0)) (`self.K2_GetActorLocation`)) -200.0)) (.y (* (`KismetMathLibrary.GetDirectionUnitVector` (`self.K2_GetActorLocation` (`GameplayStatics.GetPlayerCharacter` 0)) (`self.K2_GetActorLocation`)) -200.0)) 300.0) true true)
  (`GameplayStatics.PlaySound2D` "/Game/Assets/Cyat/Sound/cat_screech_edit_Cue.cat_screech_edit_Cue" 1.0 1.0 0.0 null null)
  (message `/Game/2DSideScrollerBP/Blueprints/BPI_Event.Stun` _returnvalue_2)
  (`self.DisableInput` _returnvalue_2 _returnvalue)
  (`KismetSystemLibrary.Delay` 0.7)
  (`self.EnableInput` _returnvalue_2 _returnvalue)
  (`PaperFlipbookComponent.SetFlipbook` (`self.PaperFlipbook`) "/Game/Assets/Space_Cyat/Idle/Space_cat.Space_cat"))

(fn `UserConstructionScript`
  (set `InterpToMovementComponent.ControlPoints` (`|MakeArray` (make `InterpControlPoint` (`self.Point A`)) (make `InterpControlPoint` (`self.Point B`))) (`self.InterpToMovement`)))